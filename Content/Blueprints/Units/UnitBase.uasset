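; UnitBase is a base unit Blueprint that supports click-to-select with a decal highlight.
; A left click toggles selection by asking the player's MainController to add or remove the unit, using decal visibility as the current selection state.
; An IsSelected event shows or hides the decal to match the selection.
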(event `self.ReceiveActorOnClicked`
  (params (ButtonPressed :type "Key Structure"))
  ;[1 1 1] When unit is clicked, add or remove from selection
  (if (== ButtonPressed "LeftMouseButton")
    (bind _asmain_controller (cast `/Game/Blueprints/Camera/MainController` (`GameplayStatics.GetPlayerController` 0)))
    (if (`SceneComponent.IsVisible` (`self.Decal`))
      (`/Game/Blueprints/Camera/MainController.RemoveUnitFromSelection` _asmain_controller self)
      (else
        (`/Game/Blueprints/Camera/MainController.AddUnitToSelection` _asmain_controller self)))))

(event `IsSelected`
  (params (IsSelected :type Boolean))
  ;[1 1 1] If unit is selected, add highlight decal. If not, remove highlight decal
  (`SceneComponent.SetVisibility` (`self.Decal`) IsSelected false))

(fn `UserConstructionScript`)