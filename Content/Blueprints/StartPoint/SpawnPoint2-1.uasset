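; Wave spawn point that sends Soldiers and Cannons toward TargetPoint2-1.
; Tick polls the TownHall's RoundNum and, when it matches NextRound, flags InRound and calls SpawnWave.
; From round two, SpawnWave fills a shuffled Stash with hidden units at random offsets, in counts that grow each round.
; EventGraph then targets, reveals and releases stashed units, with a Delay loop on unit age before removing them from Stash.
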(event `self.ReceiveBeginPlay`
  ;[1 1 1] On start, get loop goin.
  (`self.GetRoundNum`)
  (`self.IncreaseNextRound`)
  ;[1 1 1] Check if we can spawn wave. If so, spawn wave.
  (bind _canweproceed (`self.CanWeProceed` :!label _label))
  (if _canweproceed
    (`self.SetInWave` true)
    (`self.IncreaseNextRound`)
    (`self.SpawnWave`)
    ;[1 1 1] Loop through each unit
    (for _array_element (`self.Stash`)
      ;[1 1 1] Loop through all target points until we find our target
      (bind _outactors (`GameplayStatics.GetAllActorsOfClass` "/Script/Engine.TargetPoint"))
      (for _array_element_2 _outactors
        (if (`KismetStringLibrary.EqualEqual_StrStr` (`KismetSystemLibrary.GetObjectName` _array_element_2) "TargetPoint2-1")
          ;[1 1 1] Identify what unit this is
          (bind _assoldier (cast `/Game/Blueprints/AI/Soldier` _array_element)
            (:`then`
              (set `/Game/Blueprints/AI/Soldier.TargetPoint` _array_element_2 _assoldier)
              ;[1 1 1] Reveal actor
              (`self.SetActorHiddenInGame` _assoldier false)
              (set `/Game/Blueprints/AI/Soldier.CanGo` true _assoldier)
              (if (< (`self.GetGameTimeSinceCreation` _assoldier) 5.0) :!label _label_2
                (`KismetSystemLibrary.Delay` 0.2)
                (goto _label_2)
                (else
                  _)))
            (:`CastFailed`
              (bind _ascannon (cast `/Game/Blueprints/AI/Cannon` _array_element))
              (set `/Game/Blueprints/AI/Cannon.TargetPoint` _array_element_2 _ascannon)
              (`self.SetActorHiddenInGame` _ascannon false)
              (set `/Game/Blueprints/AI/Cannon.CanGo` true _ascannon)
              (if (< (`self.GetGameTimeSinceCreation` _ascannon) 5.0) :!label _label_3
                (`KismetSystemLibrary.Delay` 0.2)
                (goto _label_3)
                (else
                  _))))
          (`KismetArrayLibrary.Array_RemoveItem` (`self.Stash`) _array_element))))))

(event `self.ReceiveTick`
  (params (DeltaSeconds :type "Float (single-precision)"))
  ;[1 1 1] keep updating round num
  (`self.GetRoundNum`)
  (goto _label))

(fn `CanWeProceed`
  (returns (CanWeProceed :type Boolean))
  (if (== (`self.RoundNum`) (`self.nextRound`))
    (return true)
    (else
      (return false))))

(fn `GetRoundNum`
  (bind _returnvalue (`GameplayStatics.GetActorOfClass` "/Game/Blueprints/Structures/TownHall.TownHall_C"))
  (set `self.RoundNum` (`/Game/Blueprints/Structures/TownHall.RoundNum` _returnvalue)))

(fn `IncreaseNextRound`
  (set `self.nextRound` (+ (`self.nextRound`) 1)))

(fn `SetInWave`
  (params (`InWave?` :type Boolean))
  (bind _returnvalue (`GameplayStatics.GetActorOfClass` "/Game/Blueprints/Structures/TownHall.TownHall_C"))
  (set `/Game/Blueprints/Structures/TownHall.InRound` `InWave?` _returnvalue)
  (return))

(fn `SpawnWave`
  (bind (_returnvalue_x _returnvalue_y _returnvalue_z) (`KismetMathLibrary.BreakVector` (`self.K2_GetActorLocation`)))
  (bind (_returnvalue_x_2 _returnvalue_y_2 _returnvalue_z_2) (`KismetMathLibrary.BreakVector` (`self.K2_GetActorLocation`)))
  (bind _roundnum (`self.RoundNum`))
  (`self.GetRoundNum`)
  (if (>= (`self.RoundNum`) 2)
    ;[1 1 1] Set num units
    (set `self.HowManySoldiers` (+ 7 (* (- _roundnum 1) 2)))
    (set `self.HowManyCannons` (+ 3 (* (- _roundnum 1) 2)))
    ;[1 1 1] Loop until we have filled our stash
    (while (!= (`self.HowManySoldiers`) 0)
      ;[1 1 1] Spawn Soldier and keep hidden until ready
      (bind _returnvalue (`AIBlueprintHelperLibrary.SpawnAIFromClass` "/Game/Blueprints/AI/Soldier.Soldier_C" null (`KismetMathLibrary.MakeVector` (+ _returnvalue_x_2 (`KismetMathLibrary.RandomFloatInRange` -350.0 350.0)) (+ _returnvalue_y_2 (`KismetMathLibrary.RandomFloatInRange` -250.0 250.0)) _returnvalue_z_2) (struct) false null))
      (bind _assoldier (cast `/Game/Blueprints/AI/Soldier` _returnvalue))
      (set `/Game/Blueprints/AI/Soldier.CanGo` false _assoldier)
      (`KismetArrayLibrary.Array_Add` (`self.Stash`) _returnvalue)
      (`self.SetActorHiddenInGame` _returnvalue true)
      (set `self.HowManySoldiers` (- (`self.HowManySoldiers`) 1)))
    (while (!= (`self.HowManyCannons`) 0)
      ;[1 1 1] Spawn Cannon and keep hidden until ready
      (bind _returnvalue_2 (`AIBlueprintHelperLibrary.SpawnAIFromClass` "/Game/Blueprints/AI/Cannon.Cannon_C" null (`KismetMathLibrary.MakeVector` (+ _returnvalue_x (`KismetMathLibrary.RandomFloatInRange` -350.0 350.0)) (+ _returnvalue_y (`KismetMathLibrary.RandomFloatInRange` -250.0 250.0)) _returnvalue_z) (struct) false null))
      (bind _ascannon (cast `/Game/Blueprints/AI/Cannon` _returnvalue_2))
      (set `/Game/Blueprints/AI/Cannon.CanGo` false _ascannon)
      (`KismetArrayLibrary.Array_Add` (`self.Stash`) _returnvalue_2)
      (`self.SetActorHiddenInGame` _returnvalue_2 true)
      (set `self.HowManyCannons` (- (`self.HowManyCannons`) 1)))
    ;[1 1 1] Shuffle array for random dispersement
    (`KismetArrayLibrary.Array_Shuffle` (`self.Stash`))
    (return)
    (else
      (return))))

(fn `UserConstructionScript`)