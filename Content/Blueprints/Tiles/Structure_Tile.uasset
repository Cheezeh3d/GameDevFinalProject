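; Structure_Tile is a clickable tile marking an area where a structure can be placed.
; Hovering tints its mesh Available or Unavailable based on CanSpawnAStructure, and leaving clears the tint unless the tile is selected.
; Clicking resets all Dirt_Tile and Structure_Tile selections, then selects this tile if it can spawn a structure.
; Selection replaces any InGame widget with a new one that receives the tile as StructureArea to take over the logic.
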(event `self.StaticMesh.OnBeginCursorOver`
  (params (TouchedComponent :type "PrimitiveComponent Object Reference"))
  (bind _staticmesh (`self.StaticMesh`))
  ;[1 1 1] Change colors for when hovering over area
  (if (`self.CanSpawnAStructure`)
    (`PrimitiveComponent.SetMaterial` _staticmesh 0 "/Game/Assets/Materials/available.available")
    (else
      (`PrimitiveComponent.SetMaterial` _staticmesh 0 "/Game/Assets/Materials/unavailable.unavailable"))))

(event `self.StaticMesh.OnEndCursorOver`
  (params (TouchedComponent :type "PrimitiveComponent Object Reference"))
  ;[1 1 1] Change colors for when hovering over area
  (if (not (`self.InSelection`))
    (`PrimitiveComponent.SetMaterial` (`self.StaticMesh`) 0 null)))

(event `self.StaticMesh.OnClicked`
  (params (TouchedComponent :type "PrimitiveComponent Object Reference") (ButtonPressed :type "Key Structure"))
  ;[1 1 1] Selection logic for when we click on a structure area
  (bind _outactors (`GameplayStatics.GetAllActorsOfClass` "/Game/Blueprints/Tiles/Dirt_Tile.Dirt_Tile_C"))
  (for _array_element _outactors
    ;[1 1 1] Reset all materials for any other structure area
    (bind _asdirt_tile (cast `/Game/Blueprints/Tiles/Dirt_Tile` _array_element))
    (`PrimitiveComponent.SetMaterial` (`/Game/Blueprints/Tiles/Dirt_Tile.StaticMesh` _asdirt_tile) 0 "/Game/Assets/Map_Tiles/Beige.Beige")
    (set `/Game/Blueprints/Tiles/Dirt_Tile.InSelection` false _asdirt_tile))
  (bind _outactors_2 (`GameplayStatics.GetAllActorsOfClass` "Structure_Tile_C"))
  (for _array_element_2 _outactors_2
    (if (not (== _array_element_2 TouchedComponent))
      (bind _asstructure_tile (cast `/Game/Blueprints/Tiles/Structure_Tile` _array_element_2))
      (`self.ResetStructureArea` _asstructure_tile)))
  (if (`self.CanSpawnAStructure`)
    (set `self.InSelection` true)
    (`PrimitiveComponent.SetMaterial` (`self.StaticMesh`) 0 "/Game/Assets/Materials/available.available")
    ;[1 1 1] Reset widget to ensure we aren't stacking widgets accidentally
    (bind _foundwidgets (`WidgetBlueprintLibrary.GetAllWidgetsOfClass` "/Game/UI/InGame.InGame_C" false))
    (for _array_element_3 _foundwidgets
      (`Widget.RemoveFromParent` _array_element_3))
    (bind _returnvalue (`|CreateWidget` "/Game/UI/InGame.InGame_C"))
    (`UserWidget.AddToViewport` _returnvalue 0)
    ;[1 1 1] Set structure area for widget so widget can take over logic
    (set `/Game/UI/InGame.StructureArea` self _returnvalue)))

(fn `ResetStructureArea`
  (set `self.InSelection` false)
  (`PrimitiveComponent.SetMaterial` (`self.StaticMesh`) 0 null))

(fn `UserConstructionScript`)