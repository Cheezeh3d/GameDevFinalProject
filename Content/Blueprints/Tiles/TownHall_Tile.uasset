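; Map tile that places the Town Hall and shows its area as unavailable on cursor hover.
; On BeginPlay it spawns a TownHall actor at its transform, then nudges it up and slightly along X.
; Hovering applies the Unavailable material, and leaving clears that override unless the tile is in selection.
; ResetStructureArea drops the selection flag and clears the material override.
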(event `self.ReceiveBeginPlay`
  ;[1 1 1] Spawn Town Hall
  (bind _returnvalue (`|SpawnActorFromClass` "/Game/Blueprints/Structures/TownHall.TownHall_C" (`self.GetTransform` self) "Undefined" "OverrideRootScale" null null))
  (`self.K2_SetActorLocation` _returnvalue (+ (`self.K2_GetActorLocation` _returnvalue) (10.0 0.0 100.0)) false false))

(event `self.StaticMesh.OnBeginCursorOver`
  (params (TouchedComponent :type "PrimitiveComponent Object Reference"))
  ;[1 1 1] Change colors for when hovering over area
  (`PrimitiveComponent.SetMaterial` (`self.StaticMesh`) 0 "/Game/Assets/Materials/unavailable.unavailable"))

(event `self.StaticMesh.OnEndCursorOver`
  (params (TouchedComponent :type "PrimitiveComponent Object Reference"))
  ;[1 1 1] Change colors for when hovering over area
  (if (not (`self.InSelection`))
    (`PrimitiveComponent.SetMaterial` (`self.StaticMesh`) 0 null)))

(fn `ResetStructureArea`
  (set `self.InSelection` false)
  (`PrimitiveComponent.SetMaterial` (`self.StaticMesh`) 0 null))

(fn `UserConstructionScript`)