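; Tower structure that automatically damages TestAI, Soldier and Cannon units inside its Detect range.
; Overlap begin and end events maintain the UnitsInRange list.
; From BeginPlay, an endless Delay loop subtracts Damage from the first listed unit's Health and plays a hit sound at world origin.
; It drops that unit from the list once its remaining Health is no more than one hit's Damage.
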(event `self.Detect.OnComponentBeginOverlap`
  (params (OverlappedComponent :type "PrimitiveComponent Object Reference") (OtherActor :type "Actor Object Reference") (OtherComp :type "PrimitiveComponent Object Reference") (OtherBodyIndex :type Integer) (bFromSweep :type Boolean) (SweepResult :type "HitResult Structure (by ref)"))
  ;[1 1 1] If within radius, add enemy to range
  (bind _astest_ai (cast `/Game/Blueprints/AI/TestAI` OtherActor)
    (:`then`
      (if (not (`self.IsActorBeingDestroyed` _astest_ai))
        (`KismetArrayLibrary.Array_Add` (`self.UnitsInRange`) _astest_ai)))
    (:`CastFailed`
      (bind _assoldier (cast `/Game/Blueprints/AI/Soldier` OtherActor)
        (:`then`
          (if (not (`self.IsActorBeingDestroyed` _assoldier))
            (`KismetArrayLibrary.Array_Add` (`self.UnitsInRange`) _assoldier)))
        (:`CastFailed`
          (bind _ascannon (cast `/Game/Blueprints/AI/Cannon` OtherActor))
          (if (not (`self.IsActorBeingDestroyed` _ascannon))
            (`KismetArrayLibrary.Array_Add` (`self.UnitsInRange`) _ascannon)))))))

(event `self.Detect.OnComponentEndOverlap`
  (params (OverlappedComponent :type "PrimitiveComponent Object Reference") (OtherActor :type "Actor Object Reference") (OtherComp :type "PrimitiveComponent Object Reference") (OtherBodyIndex :type Integer))
  ;[1 1 1] Remove enemy from range when exits range
  (bind _astest_ai (cast `/Game/Blueprints/AI/TestAI` OtherActor)
    (:`then`
      (if (not (`self.IsActorBeingDestroyed` _astest_ai))
        (`KismetArrayLibrary.Array_RemoveItem` (`self.UnitsInRange`) _astest_ai)))
    (:`CastFailed`
      (bind _assoldier (cast `/Game/Blueprints/AI/Soldier` OtherActor)
        (:`then`
          (if (not (`self.IsActorBeingDestroyed` _assoldier))
            (`KismetArrayLibrary.Array_RemoveItem` (`self.UnitsInRange`) _assoldier)))
        (:`CastFailed`
          (bind _ascannon (cast `/Game/Blueprints/AI/Cannon` OtherActor))
          (if (not (`self.IsActorBeingDestroyed` _ascannon))
            (`KismetArrayLibrary.Array_RemoveItem` (`self.UnitsInRange`) _ascannon)))))))

(event `self.ReceiveBeginPlay`
  ;[1 1 1] Attack first target in list
  (`KismetSystemLibrary.Delay` 0.7 :!label _label)
  (for (_array_element _array_index) (`self.UnitsInRange`)
    (if (== _array_index 0)
      (bind _astest_ai (cast `/Game/Blueprints/AI/TestAI` _array_element)
        (:`then`
          (if (not (`self.IsActorBeingDestroyed` _astest_ai))
            (bind _returnvalue (- (`/Game/Blueprints/AI/TestAI.Health` _astest_ai) (`self.Damage`)))
            (set `/Game/Blueprints/AI/TestAI.Health` _returnvalue _astest_ai)
            (`GameplayStatics.SpawnSoundAtLocation` "/Game/Sound/Hit.Hit" (0.0 0.0 0.0) (struct) 1.0 1.0 0.0 null null)
            (if (<= _returnvalue 0)
              (`KismetArrayLibrary.Array_Remove` (`self.UnitsInRange`))
              (break))))
        (:`CastFailed`
          (bind _assoldier (cast `/Game/Blueprints/AI/Soldier` _array_element)
            (:`then`
              (if (not (`self.IsActorBeingDestroyed` _assoldier))
                (bind _returnvalue_2 (- (`/Game/Blueprints/AI/Soldier.Health` _assoldier) (`self.Damage`)))
                (set `/Game/Blueprints/AI/Soldier.Health` _returnvalue_2 _assoldier)
                (`GameplayStatics.SpawnSoundAtLocation` "/Game/Sound/Hit.Hit" (0.0 0.0 0.0) (struct) 1.0 1.0 0.0 null null)
                (if (<= _returnvalue_2 0)
                  (`KismetArrayLibrary.Array_Remove` (`self.UnitsInRange`))
                  (break))))
            (:`CastFailed`
              (bind _ascannon (cast `/Game/Blueprints/AI/Cannon` _array_element))
              (if (not (`self.IsActorBeingDestroyed` _ascannon))
                (bind _returnvalue_3 (- (`/Game/Blueprints/AI/Cannon.Health` _ascannon) (`self.Damage`)))
                (set `/Game/Blueprints/AI/Cannon.Health` _returnvalue_3 _ascannon)
                (`GameplayStatics.SpawnSoundAtLocation` "/Game/Sound/Hit.Hit" (0.0 0.0 0.0) (struct) 1.0 1.0 0.0 null null)
                (if (<= _returnvalue_3 0)
                  (`KismetArrayLibrary.Array_Remove` (`self.UnitsInRange`))
                  (break)))))))))
  (goto _label))

(fn `UserConstructionScript`)