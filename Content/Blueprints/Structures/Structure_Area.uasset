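; Structure_Area is a clickable placement area actor that shows through its mesh material whether a structure can be spawned on it.
; Cursor hover switches the StaticMesh to the Available or Unavailable material based on CanSpawnAStructure.
; Clicking applies Available when spawning is allowed and otherwise clears the material override, as does the cursor leaving.
; The graph only handles this visual feedback and contains no spawning logic.
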(event `self.StaticMesh.OnBeginCursorOver`
  (params (TouchedComponent :type "PrimitiveComponent Object Reference"))
  (bind _staticmesh (`self.StaticMesh`))
  (if (`self.CanSpawnAStructure`)
    (`PrimitiveComponent.SetMaterial` _staticmesh 0 "/Game/Assets/Materials/available.available")
    (else
      (`PrimitiveComponent.SetMaterial` _staticmesh 0 "/Game/Assets/Materials/unavailable.unavailable"))))

(event `self.StaticMesh.OnClicked`
  (params (TouchedComponent :type "PrimitiveComponent Object Reference") (ButtonPressed :type "Key Structure"))
  (bind _staticmesh (`self.StaticMesh`))
  (if (`self.CanSpawnAStructure`)
    (`PrimitiveComponent.SetMaterial` _staticmesh 0 "/Game/Assets/Materials/available.available")
    (else
      (`PrimitiveComponent.SetMaterial` _staticmesh 0 null :!label _label))))

(event `self.StaticMesh.OnEndCursorOver`
  (params (TouchedComponent :type "PrimitiveComponent Object Reference"))
  (goto _label))

(fn `UserConstructionScript`)