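; Town hall structure that acts as the game manager for a round-based defense game, ending play on defeat or victory.
; A delayed loop adds Energy every five seconds during rounds.
; Tick checks Health for a loss, ends rounds when no Soldiers or visible Cannons remain, and declares a win at round 4 between rounds.
; Helper functions swap InGame, win, lose and pause widgets and set game pause.
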(event `self.ReceiveBeginPlay`
  ;[1 1 1] Loop to give energy every 1 second during a round
  (`KismetSystemLibrary.Delay` 5.0 :!label _label)
  (if (`self.InRound`)
    (set `self.Energy` (+ (`self.Energy`) 5))
    (goto _label)
    (else
      (goto _label))))

(event `self.ReceiveTick`
  (params (DeltaSeconds :type "Float (single-precision)"))
  ;[1 1 1] Check to see if our health ran out. If so, end game.
  (if (<= (`self.Health`) 0)
    (`self.ChangeUIGameOver`)
    (else
      ;[1 1 1] Check if all enemies dead within one round. If so, change round number, prep for next round
      (if (`self.InRound`)
        (bind _alive_ (`self.CheckIfEnemyAlive`))
        (if (not _alive_)
          (set `self.InRound` false))
        (else
          ;[1 1 1] If we get past three round, we win, so change UI to win screen
          (if (== (`self.RoundNum`) 4)
            (`self.ChangeUIGameWin`)))))))

(fn `ChangeUIGameOver`
  (bind _foundwidgets (`WidgetBlueprintLibrary.GetAllWidgetsOfClass` "/Game/UI/InGame.InGame_C" false))
  (for _array_element _foundwidgets
    (`Widget.RemoveFromParent` _array_element))
  (bind _returnvalue (`|CreateWidget` "/Game/UI/LoseScreen.LoseScreen_C"))
  (`UserWidget.AddToViewport` _returnvalue 0)
  (`GameplayStatics.SetGamePaused` true)
  (`self.K2_DestroyActor`))

(fn `ChangeUIGameWin`
  (bind _foundwidgets (`WidgetBlueprintLibrary.GetAllWidgetsOfClass` "/Game/UI/InGame.InGame_C" false))
  (for _array_element _foundwidgets
    (`Widget.RemoveFromParent` _array_element))
  (bind _returnvalue (`|CreateWidget` "/Game/UI/WinScreen.WinScreen_C"))
  (`UserWidget.AddToViewport` _returnvalue 0)
  (`GameplayStatics.SetGamePaused` true)
  (`self.K2_DestroyActor`))

(fn `CheckIfEnemyAlive`
  (returns (`Alive?` :type Boolean))
  (bind _outactors (`GameplayStatics.GetAllActorsOfClass` "/Game/Blueprints/AI/Soldier.Soldier_C"))
  (bind _outactors_2 (`GameplayStatics.GetAllActorsOfClass` "/Game/Blueprints/AI/Cannon.Cannon_C"))
  (if (> (+ (`KismetArrayLibrary.Array_Length` _outactors_2) (`KismetArrayLibrary.Array_Length` _outactors)) 0)
    (for _array_element _outactors_2
      (if (`self.IsActorBeingDestroyed` _array_element)
        _
        (elif (not (`Actor.bHidden` _array_element))
          (return true))))
    (for _array_element_2 _outactors
      (if (not (`self.IsActorBeingDestroyed` _array_element_2))
        (return true)))
    (return false)
    (else
      (return false))))

(fn `Pause,Unpause`
  (if (`GameplayStatics.IsGamePaused`)
    (bind _foundwidgets (`WidgetBlueprintLibrary.GetAllWidgetsOfClass` "/Game/UI/PauseScreen.PauseScreen_C" false))
    (for _array_element _foundwidgets
      (`Widget.RemoveFromParent` _array_element))
    (bind _returnvalue (`|CreateWidget` "/Game/UI/InGame.InGame_C"))
    (`UserWidget.AddToViewport` _returnvalue 0)
    (`GameplayStatics.SetGamePaused` false)
    (else
      (bind _foundwidgets_2 (`WidgetBlueprintLibrary.GetAllWidgetsOfClass` "/Game/UI/InGame.InGame_C" false))
      (for _array_element_2 _foundwidgets_2
        (`Widget.RemoveFromParent` _array_element_2))
      (bind _returnvalue_2 (`|CreateWidget` "/Game/UI/PauseScreen.PauseScreen_C"))
      (`UserWidget.AddToViewport` _returnvalue_2 0)
      (`GameplayStatics.SetGamePaused` true))))

(fn `UserConstructionScript`)