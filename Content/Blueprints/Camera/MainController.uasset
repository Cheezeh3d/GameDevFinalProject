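; Player controller that drives a MainCamera with mouse-wheel zoom and screen-edge panning.
; On BeginPlay it caches the view target as MainCamera and enables a locked, visible cursor with click and hover events.
; The wheel axis adjusts a clamped zoom factor that sets spring arm length.
; MouseX/MouseY axes feed the ScreenEdgeMovement macro, which turns cursor proximity to viewport edges into sensitivity-scaled local camera offsets.
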(event `self.ReceiveBeginPlay`
  ;[1 1 1] Set main camera, enable mouse cursor
  (`WidgetBlueprintLibrary.SetInputMode_GameAndUIEx` self null "LockAlways" false)
  (bind _asmain_camera (cast `/Game/Blueprints/Camera/MainCamera` (`self.GetViewTarget`)))
  (set `self.MainCamera` _asmain_camera)
  (set `self.bShowMouseCursor` true)
  (set `self.bEnableClickEvents` true)
  (set `self.bEnableMouseOverEvents` true))

(event `InputAxisKey|MouseWheelAxis`
  (params (AxisValue :type "Float (single-precision)"))
  ;[1 1 1] Logic for zooming camera in and out.
  (bind _output_get (set `self.ZoomFactor` (`KismetMathLibrary.FClamp` (+ (* AxisValue -1.0) (`self.ZoomFactor`)) 0.0 10.0)))
  (set `SpringArmComponent.TargetArmLength` (+ (* _output_get 200.0) 300.0) (`/Game/Blueprints/Camera/MainCamera.SpringArm` (`self.MainCamera`))))

(event `InputAxisKey|MouseX`
  (params (AxisValue :type "Float (single-precision)"))
  ;[1 1 1] Move Camera
  (bind (_deltaxspeed _deltayspeed) (`self.ScreenEdgeMovement` :!label _label)
    (:`ReturnNode`
      (`self.K2_AddActorLocalOffset` (`self.MainCamera`) (`KismetMathLibrary.MakeVector` _deltaxspeed _deltayspeed) false false))))

(event `InputAxisKey|MouseY`
  (params (AxisValue :type "Float (single-precision)"))
  ;[1 1 1] Move Camera
  (goto _label :!via `MouseY`))

(fn `UserConstructionScript`)