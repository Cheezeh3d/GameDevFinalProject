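; HUD Blueprint that provides drag-box selection of units, drawing a translucent red rectangle on screen.
; StartSelection records the scaled mouse position as the first corner.
; While drawing, DrawHUD updates the opposite corner, draws the rectangle and gathers UnitBase actors inside it each frame.
; StopSelection ends drawing, clears the MainController's unit selection and adds the gathered units to it.
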(event `self.ReceiveBeginPlay`
  ;[1 1 1] At start, store main controller instance as variable
  (bind _asmain_controller (cast `/Game/Blueprints/Camera/MainController` (`GameplayStatics.GetPlayerController` 0)))
  (set `self.As MainController` _asmain_controller))

(event `/Game/Blueprints/Camera/SelectionInterface.StartSelection`
  ;[1 1 1] If left mouse was held, we start selection, and start drawing rectangle
  (bind _returnvalue (`WidgetLayoutLibrary.GetMousePositionOnViewport`))
  (bind (_returnvalue_x _returnvalue_y) (`KismetMathLibrary.BreakVector2D` (* _returnvalue (`WidgetLayoutLibrary.GetViewportScale`))))
  (set `self.PointA` (`KismetMathLibrary.MakeVector2D` _returnvalue_x _returnvalue_y))
  (set `self.isDrawing` true))

(event `/Game/Blueprints/Camera/SelectionInterface.StopSelection`
  ;[1 1 1] If left mouse button was released, stop drawing rectangle.
  (set `self.isDrawing` false)
  (`/Game/Blueprints/Camera/MainController.ClearUnitSelection` (`self.As MainController`))
  (for _array_element (`self.SelectionOfActors`)
    (bind _asunit_base (cast `/Game/Blueprints/Units/UnitBase` _array_element))
    (`/Game/Blueprints/Camera/MainController.AddUnitToSelection` (`self.As MainController`) _asunit_base)))

(event `self.ReceiveDrawHUD`
  (params (SizeX :type Integer) (SizeY :type Integer))
  (bind (_pointa_x _pointa_y) (`KismetMathLibrary.BreakVector2D` (`self.PointA`)))
  (bind (_pointb_x _pointb_y) (`KismetMathLibrary.BreakVector2D` (`self.PointB`)))
  ;[1 1 1] Logic for drawing rectangle on screen. Add all units within rectangle into selection
  (if (`self.isDrawing`)
    (bind _returnvalue (`WidgetLayoutLibrary.GetMousePositionOnViewport`))
    (bind (_returnvalue_x _returnvalue_y) (`KismetMathLibrary.BreakVector2D` (* _returnvalue (`WidgetLayoutLibrary.GetViewportScale`))))
    (set `self.PointB` (`KismetMathLibrary.MakeVector2D` _returnvalue_x _returnvalue_y))
    (`self.DrawRect` (struct :`R` 1.0 :`A` 0.368) _pointa_x _pointa_y (- _pointb_x _pointa_x) (- _pointb_y _pointa_y))
    (set `self.SelectionOfActors` (`self.GetActorsInSelectionRectangle` "/Game/Blueprints/Units/UnitBase.UnitBase_C" (`self.PointA`) (`self.PointB`)))))

(fn `UserConstructionScript`)