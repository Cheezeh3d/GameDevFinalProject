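; Cannon is an AI-moved pawn that travels to a target point and repeatedly damages the TownHall.
; After spawning it waits briefly for its TargetPoint to arrive, then uses AI MoveTo toward the first actor of that TargetPoint's class.
; On a successful move, a looping timer fires AttackTownHall, which directly decrements the Health of the TownHall found by class lookup.
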(event `AttackTownHall`
  ;[1 1 1] Attack TownHall
  (bind _returnvalue (`GameplayStatics.GetActorOfClass` "/Game/Blueprints/Structures/TownHall.TownHall_C"))
  (set `/Game/Blueprints/Structures/TownHall.Health` (- (`/Game/Blueprints/Structures/TownHall.Health` _returnvalue) 1) _returnvalue))

(event `self.ReceiveBeginPlay`
  ;[1 1 1] when spawned, wait a second to receive the targetpoint, then move toward it.
  (`KismetSystemLibrary.Delay` 1.0)
  (bind _outactors (`GameplayStatics.GetAllActorsOfClass` (`GameplayStatics.GetObjectClass` (`self.TargetPoint`))))
  (`|AIMoveTo` self (0.0 0.0 0.0) (`|GetArrayItem` _outactors)
    (:`OnSuccess`
      ;[1 1 1] Attack TownHall
      (`KismetSystemLibrary.K2_SetTimerDelegate` (delegate `AttackTownHall`) 0.5 true))))

(fn `UserConstructionScript`)