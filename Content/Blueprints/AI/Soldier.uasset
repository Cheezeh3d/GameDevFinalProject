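; Soldier AI unit that advances on a target point, attacks obstacles and the TownHall, and destroys itself when its Health runs out.
; Tick checks Health and, once CanGo is set, issues AIMoveTo toward TargetPoint.
; Reaching the target starts a delayed loop that subtracts Damage from TownHall Health with a sound.
; Capsule hits on Barricades start a similar loop, which resumes movement once the barricade is being destroyed.
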(event `self.ReceiveTick`
  (params (DeltaSeconds :type "Float (single-precision)"))
  ;[1 1 1] If health drops below zero, kill actor
  (if (<= (`self.Health`) 0)
    (`self.K2_DestroyActor`)
    (else
      ;[1 1 1] when spawned, wait a second to receive the targetpoint, then move toward it.
      (if (`self.CanGo`)
        (`|AIMoveTo` self (0.0 0.0 0.0) (`self.TargetPoint`) :!label _label
          (:`OnSuccess`
            ;[1 1 1] Attack TownHall
            (`KismetSystemLibrary.Delay` 1.0 :!label _label_2)
            (bind _returnvalue (`GameplayStatics.GetActorOfClass` "/Game/Blueprints/Structures/TownHall.TownHall_C"))
            (set `/Game/Blueprints/Structures/TownHall.Health` (- (`/Game/Blueprints/Structures/TownHall.Health` _returnvalue) (`self.Damage`)) _returnvalue)
            (`GameplayStatics.PlaySoundAtLocation` null (0.0 0.0 0.0) (struct) 1.0 1.0 0.0 null null null)
            (goto _label_2)))))))

(event `self.CapsuleComponent.OnComponentHit`
  (params (HitComponent :type "PrimitiveComponent Object Reference") (OtherActor :type "Actor Object Reference") (OtherComp :type "PrimitiveComponent Object Reference") (NormalImpulse :type "Vector Structure") (Hit :type "HitResult Structure (by ref)"))
  ;[1 1 1] Check if we hit a barracade. If so, attack it until it's destroyed. Then, progress forward.
  (bind _asbarricades (cast `/Game/Blueprints/Structures/Barricades` OtherActor))
  (if (`self.IsActorBeingDestroyed` _asbarricades) :!label _label_3
    (goto _label)
    (else
      (`KismetSystemLibrary.Delay` 0.5)
      (set `/Game/Blueprints/Structures/Barricades.Health` (- (`/Game/Blueprints/Structures/Barricades.Health` _asbarricades) (`self.Damage`)) _asbarricades)
      (`GameplayStatics.PlaySoundAtLocation` null (0.0 0.0 0.0) (struct) 1.0 1.0 0.0 null null null)
      (goto _label_3))))

(fn `UserConstructionScript`)